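; Interactive spring that launches the player upward.
; Interact calls LaunchCharacter on the passed player with a vertical force variable, then plays the Paper2D flipbook from the start.
; The construction script runs the parent's, then sets flipbook looping from the AutoPlay flag.
; BeginPlay only defers to the parent, and the Blueprint uses no Tick or overlap logic of its own.
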(event EventBeginPlay
  (|CallParentFunction))

(event Collision|EventActorBeginOverlap
  (params (OtherActor :type Actor%20Object%20Reference)))

(event EventTick
  (params (DeltaSeconds :type Float%20%28single-precision%29)))

(fn ConstructionScript
  (|CallParentFunction)
  (Components|Timeline|SetLooping (Variables|Default|GetPaperFlipbook) (Variables|Default|GetAutoPlay)))

(fn Interact
  (params (PlayerRef :type BP%20Player%20Base%20Object%20Reference))
  (Character|LaunchCharacter PlayerRef (Math|Vector|MakeVector 0.0 0.0 (Variables|Default|GetLauchForce)) false false)
  (Components|Timeline|PlayfromStart (Variables|Default|GetPaperFlipbook)))