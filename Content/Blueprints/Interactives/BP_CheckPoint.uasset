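; BP_CheckPoint is an interactive checkpoint with a zone that tracks whether the player is inside it.
; Overlap events on InteractiveCollider set InCheckPointZone for BP_PlayerBase actors.
; ActivateCheckPoint fully heals the player, calls the respawn-all-enemies dispatcher, and marks the checkpoint as activated.
; The parent construction script call is left unconnected.
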(event OnComponentBeginOverlap(InteractiveCollider)
  (params (OverlappedComponent :type Primitive%20Component%20Object%20Reference) (OtherActor :type Actor%20Object%20Reference) (OtherComp :type Primitive%20Component%20Object%20Reference) (OtherBodyIndex :type Integer) (bFromSweep :type Boolean) (SweepResult :type Hit%20Result%20Structure%20%28by%20ref%29))
  ;[1 1 1] Check if in/out of zone
  (Utilities|Casting|CastToBP_PlayerBase OtherActor)
  (Variables|Default|SetInCheckPointZone true))

(event OnComponentEndOverlap(InteractiveCollider)
  (params (OverlappedComponent :type Primitive%20Component%20Object%20Reference) (OtherActor :type Actor%20Object%20Reference) (OtherComp :type Primitive%20Component%20Object%20Reference) (OtherBodyIndex :type Integer))
  ;[1 1 1] Check if in/out of zone
  (Utilities|Casting|CastToBP_PlayerBase OtherActor)
  (Variables|Default|SetInCheckPointZone false))

(fn ConstructionScript)

(fn ActivateCheckPoint
  (Utilities|FlowControl|Sequence
    (:then_0
      (bind _asbp_player_base (Utilities|Casting|CastToBP_PlayerBase (Game|GetPlayerCharacter 0)))
      (Default|FullHeal _asbp_player_base)
      (Default|CallRespawnAllEnemiesDispatcher))
    (:then_1
      (Variables|Default|SetCheckPointActivated true))))