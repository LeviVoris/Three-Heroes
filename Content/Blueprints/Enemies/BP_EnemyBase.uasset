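; Base enemy Blueprint that tracks health and death state from incoming damage.
; Construction sets Health to DefaultHealth, and AnyDamage subtracts damage within a clamped range, calling EnemyDied at zero if not already flagged dead.
; Any other hit clears EnemyIsDead, including a hit on an already dead enemy.
; EnemyDied is empty, and Respawn only checks the dead flag, with an unconnected SpawnActor node left in its graph.
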(event Game|Damage|EventAnyDamage
  (params (Damage :type Float%20%28single-precision%29) (DamageType :type Damage%20Type%20Object%20Reference) (InstigatedBy :type Controller%20Object%20Reference) (DamageCauser :type Actor%20Object%20Reference))
  ;[1 1 1] Enemy Health Management
  (Variables|Default|SetHealth (Math|Float|Clamp(Float) (- (Variables|Default|GetHealth) Damage) 0.0 (Variables|Default|GetDefaultHealth)))
  (if (and (<= (Variables|Default|GetHealth) 0.0) (not (Variables|Default|GetEnemyIsDead)))
    (Variables|Default|SetEnemyIsDead true)
    (CallFunction|EnemyDied)
    (else
      (Variables|Default|SetEnemyIsDead false))))

(fn ConstructionScript
  (Variables|Default|SetHealth (Variables|Default|GetDefaultHealth)))

(fn EnemyDied)

(fn Respawn
  (if (Variables|Default|GetEnemyIsDead)
    _))