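; BP_EnemyBat is a sprite-based enemy that flies left or right along world X, starting in a random direction.
; Tick applies constant movement input, and capsule hits on non-player actors with an X normal reverse it and mirror the sprite's X scale.
; A DoOnce reset after a short delay debounces turns.
; Death destroys the actor, while Respawn spawns a new bat at its transform if dead, without calling the parent.
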(event OnComponentHit(CapsuleComponent)
  (params (HitComponent :type Primitive%20Component%20Object%20Reference) (OtherActor :type Actor%20Object%20Reference) (OtherComp :type Primitive%20Component%20Object%20Reference) (NormalImpulse :type Vector :default "0, 0, 0") (Hit :type Hit%20Result%20Structure%20%28by%20ref%29))
  ;[1 1 1] Don't change direction when player hit
  (if (!= OtherActor "/Game/Blueprints/BP_PlayerBase.BP_PlayerBase")
    (if (!= (.X (Math|Vector|BreakVector (.normal Hit))) 0.0)
      (Utilities|FlowControl|DoOnce false
        (:Completed
          (Variables|Default|SetBMoveRight (not (Variables|Default|GetBMoveRight)))
          (CallFunction|ToggleFacingDirection)
          (Utilities|FlowControl|Delay 0.1)
          (CallFunction|ResetDirectionChangeCheck))))))

(event Custom|ResetDirectionChangeCheck
  (Utilities|FlowControl|DoOnce false) ; enters at Reset
)

(event EventTick
  (params (DeltaSeconds :type Float%20%28single-precision%29))
  ;[1 1 1] Applied Movement input
  (Pawn|Input|AddMovementInput "1.000000,0.000000,0.000000" (select (Variables|Default|GetBMoveRight) 1.0 -1.0) false))

(event EventBeginPlay
  ;[1 1 1] Random Left or Right Control via Bool
  (Variables|Default|SetBMoveRight (Math|Random|RandomBool))
  (CallFunction|ToggleFacingDirection))

(fn ConstructionScript
  (|CallParentFunction))

(fn EnemyDied
  (|CallParentFunction)
  (Actor|DestroyActor))

(fn ToggleFacingDirection
  (bind _sprite (Variables|Default|GetSprite))
  (bind _returnvalue (Transformation|GetWorldScale _sprite))
  ;[1 1 1] Control Bat Facing Direction
  (Transformation|SetWorldScale3D (Variables|Default|GetSprite) (Math|Vector|MakeVector (* (Math|Float|Absolute(Float) (.x _returnvalue)) (Math|Float|SelectFloat -1.0 1.0 (Variables|Default|GetBMoveRight))) (.y _returnvalue) (.z _returnvalue))))

(fn Respawn
  (if (Variables|Default|GetEnemyIsDead)
    (Game|SpawnActorfromClass "BP_EnemyBat_C" (Transformation|GetActorTransform) "Undefined" 0 0)))